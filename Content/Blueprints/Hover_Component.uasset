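; Hover component that keeps its owning actor floating above surfaces using physics forces.
; On initialize it enables physics simulation on the owner's first primitive component.
; Each tick it traces straight down from its own location and, on a hit, pushes that primitive along the surface normal, with force fading linearly to zero at full trace length.
; A hit also applies linear and angular damping, which is never reset on a miss.
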(event EventTick
  (params (DeltaSeconds :type Float%20%28single-precision%29))
  (bind _returnvalue (Transformation|GetWorldLocation))
  ;[1 1 1] Hover above the ground
  (bind (_outhit _returnvalue_2) (Collision|LineTraceByChannel _returnvalue (- _returnvalue (Math|Vector|MakeVector 0.0 0.0 (Variables|Default|GetTraceLength))) "TraceTypeQuery1" false 0 "None")) ; Cast to floor
  (if _returnvalue_2 ; If we hit something
    (Physics|AddForce (Variables|Default|GetPrimitiveComponentRef) (* (.ImpactNormal (Collision|BreakHitResult _outhit)) (Math|Float|Lerp (Variables|Default|GetHoverForce) 0.0 (/ (Math|Vector|VectorLength (- (.Location (Collision|BreakHitResult _outhit)) (Transformation|GetWorldLocation))) (Variables|Default|GetTraceLength)))) "None")
    (Class|PrimitiveComponent|SetLinearDamping (Variables|Default|GetPrimitiveComponentRef) (Variables|Default|GetLinearDampAmount))
    (Class|PrimitiveComponent|SetAngularDamping (Variables|Default|GetPrimitiveComponentRef) (Variables|Default|GetAngularDampAmount))))

(event EventInitializeComponent
  ;[1 1 1] Set physics and get ref to primitive component
  (bind _output_get (Variables|Default|SetPrimitiveComponentRef (Utilities|Array|Get(acopy) (Actor|GetComponentsByClass (Components|GetOwner) "/Script/Engine.PrimitiveComponent"))))
  (Physics|SetSimulatePhysics _output_get true))